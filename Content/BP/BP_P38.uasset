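; BP_P38 is a player-controlled P-38 aircraft pawn that flies continuously forward and fires missiles.
; Tick feeds movement input along the actor's forward vector, scaled by ScaleValue, which the Boost input raises while held and lowers on release.
; Pitch and Roll axes rotate the actor locally using delta time and P38Speed, while Tick also spins both propeller meshes.
; Fire spawns a BP_Missile at the Arrow component's world transform.
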(event EventTick
  (params (DeltaSeconds :type Float%20%28single-precision%29))
  (Utilities|FlowControl|Sequence
    (:then_0
      ;[1 1 1] 비행기 앞으로 이동
      (Pawn|Input|AddMovementInput (Transformation|GetActorForwardVector) (Variables|Default|GetScale%20Value) false))
    (:then_1
      ;[1 1 1] 프로펠러
      (Transformation|AddLocalRotation (Variables|Default|GetSM_P38_Propeller_Left) (Math|Rotator|MakeRotator (* (Utilities|Time|GetWorldDeltaSeconds) (Variables|Default|GetPropeller_Speed)) 0.0 0.0) false false))
    (:then_2
      (Transformation|AddLocalRotation (Variables|Default|GetSM_P38_Propeller_Right) (Math|Rotator|MakeRotator (* (Utilities|Time|GetWorldDeltaSeconds) (Variables|Default|GetPropeller_Speed)) 0.0 0.0) false false))))

(event Input|ActionEvents|InputActionFire
  (params (Key :type Key%20Structure :default "None"))
  (:Pressed
    (Game|SpawnActorfromClass "/Game/BP/BP_Missile.BP_Missile_C" (Transformation|GetWorldTransform (Variables|Default|GetArrow)) "Undefined" 0 0)))

(event Input|ActionEvents|InputActionBoost
  (params (Key :type Key%20Structure :default "None"))
  (:Pressed
    (Variables|Default|SetScale%20Value 1.0))
  (:Released
    (Variables|Default|SetScale%20Value 0.5)))

(event Input|AxisEvents|InputAxisPitch
  (params (AxisValue :type Float%20%28single-precision%29))
  (Transformation|AddActorLocalRotation (Math|Rotator|MakeRotator 0.0 (* AxisValue (Utilities|Time|GetWorldDeltaSeconds) (Variables|Default|GetP38_Speed)) 0.0) false false))

(event Input|AxisEvents|InputAxisRoll
  (params (AxisValue :type Float%20%28single-precision%29))
  (Transformation|AddActorLocalRotation (Math|Rotator|MakeRotator (* AxisValue (Utilities|Time|GetWorldDeltaSeconds) (Variables|Default|GetP38_Speed)) 0.0 0.0) false false))

(fn ConstructionScript)